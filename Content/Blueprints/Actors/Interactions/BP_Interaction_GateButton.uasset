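; BP_Interaction_GateButton is an interaction actor that opens a referenced gate, but only after it has been enabled.
; CanOpen is set to false at BeginPlay and to true by the TurnOn event.
; Interact checks that Gate is valid and CanOpen is true, then casts Gate to BP_Gate and calls OpenGate.
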(event Custom|TurnOn
  (Variables|Default|SetCanOpen true))

(event EventBeginPlay
  (|CallParentFunction)
  (Variables|Default|SetCanOpen false))

(event Collision|EventActorBeginOverlap
  (params (OtherActor :type Actor%20Object%20Reference))
  (|CallParentFunction OtherActor) ; This node is disabled and will not be called.\nDrag off pins to build functionality.
)

(event EventTick
  (params (DeltaSeconds :type Float%20%28single-precision%29))
  (|CallParentFunction DeltaSeconds) ; This node is disabled and will not be called.\nDrag off pins to build functionality.
)

(event EventInteract
  (bind _gate (Variables|Default|GetGate))
  ;[1 1 1] Light Switch sets visibility of light (declared in details) on and off according to current visibility.
  (Utilities|IsValid _gate
    (:Is%20Valid
      (if (Variables|Default|GetCanOpen)
        (bind _asbp_gate (Utilities|Casting|CastToBP_Gate _gate))
        (Default|OpenGate _asbp_gate)))))

(fn ConstructionScript
  (|CallParentFunction))