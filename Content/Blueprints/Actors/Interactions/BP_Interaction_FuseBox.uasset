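; Fuse box interaction actor that lets the player switch on power for a linked gate button.
; Entering its box shows a hint on the player based on the linked Power's CanOpen flag, enabling input only while power is off.
; Interact casts Power to BP_Interaction_GateButton, calls TurnOn and updates the hint.
; Leaving the box clears the hint and disables input.
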(event OnComponentEndOverlap(Box)
  (params (OverlappedComponent :type Primitive%20Component%20Object%20Reference) (OtherActor :type Actor%20Object%20Reference) (OtherComp :type Primitive%20Component%20Object%20Reference) (OtherBodyIndex :type Integer))
  (Variables|/Game/Blueprints/Game/Level1/L1_Character.L1_Character_C|SetHintMessage (Variables|Default|GetPlayerRef) "")
  (Input|DisableInput (Game|GetPlayerController 0)))

(event OnComponentBeginOverlap(Box)
  (params (OverlappedComponent :type Primitive%20Component%20Object%20Reference) (OtherActor :type Actor%20Object%20Reference) (OtherComp :type Primitive%20Component%20Object%20Reference) (OtherBodyIndex :type Integer) (bFromSweep :type Boolean) (SweepResult :type Hit%20Result%20Structure%20%28by%20ref%29))
  (bind _returnvalue (Game|GetPlayerController 0))
  (bind _playerref (Variables|Default|GetPlayerRef))
  (if (Variables|/Game/Blueprints/Actors/Interactions/BP_Interaction_GateButton.BP_Interaction_GateButton_C|GetCanOpen (Variables|Default|GetPower))
    (Variables|/Game/Blueprints/Game/Level1/L1_Character.L1_Character_C|SetHintMessage _playerref "Power is on")
    (Input|DisableInput _returnvalue)
    (else
      (Variables|/Game/Blueprints/Game/Level1/L1_Character.L1_Character_C|SetHintMessage _playerref "Press E to turn on the power")
      (Input|EnableInput _returnvalue))))

(event EventBeginPlay
  (|CallParentFunction) ; This node is disabled and will not be called.\nDrag off pins to build functionality.
)

(event Collision|EventActorBeginOverlap
  (params (OtherActor :type Actor%20Object%20Reference))
  (|CallParentFunction OtherActor) ; This node is disabled and will not be called.\nDrag off pins to build functionality.
)

(event EventTick
  (params (DeltaSeconds :type Float%20%28single-precision%29))
  (|CallParentFunction DeltaSeconds) ; This node is disabled and will not be called.\nDrag off pins to build functionality.
)

(event EventInteract
  (bind _power (Variables|Default|GetPower))
  ;[1 1 1] Light Switch sets visibility of light (declared in details) on and off according to current visibility.
  (Utilities|IsValid _power
    (:Is%20Valid
      (bind _asbp_interaction_gate_button (Utilities|Casting|CastToBP_Interaction_GateButton _power))
      (Default|Turnon _asbp_interaction_gate_button)
      (Variables|/Game/Blueprints/Game/Level1/L1_Character.L1_Character_C|SetHintMessage (Variables|Default|GetPlayerRef) "Power is on"))))

(fn ConstructionScript
  (|CallParentFunction))