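; BP_Interaction_Readable is a readable interaction actor that shows note text to the player through a proximity trigger.
; Overlapping its Box copies NoteText into the HintMessage on PlayerRef and enables input on the actor for player controller 0.
; Ending the overlap clears the message and disables input.
; The graph handles no input events itself and does not check which actor overlaps.
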(event OnComponentEndOverlap(Box)
  (params (OverlappedComponent :type Primitive%20Component%20Object%20Reference) (OtherActor :type Actor%20Object%20Reference) (OtherComp :type Primitive%20Component%20Object%20Reference) (OtherBodyIndex :type Integer))
  (Variables|/Game/Blueprints/Game/Level1/L1_Character.L1_Character_C|SetHintMessage (Variables|Default|GetPlayerRef) "")
  (Input|DisableInput (Game|GetPlayerController 0)))

(event OnComponentBeginOverlap(Box)
  (params (OverlappedComponent :type Primitive%20Component%20Object%20Reference) (OtherActor :type Actor%20Object%20Reference) (OtherComp :type Primitive%20Component%20Object%20Reference) (OtherBodyIndex :type Integer) (bFromSweep :type Boolean) (SweepResult :type Hit%20Result%20Structure%20%28by%20ref%29))
  (Variables|/Game/Blueprints/Game/Level1/L1_Character.L1_Character_C|SetHintMessage (Variables|Default|GetPlayerRef) (Variables|Default|GetNoteText))
  (Input|EnableInput (Game|GetPlayerController 0)))

(event EventBeginPlay
  (|CallParentFunction) ; This node is disabled and will not be called.\nDrag off pins to build functionality.
)

(event Collision|EventActorBeginOverlap
  (params (OtherActor :type Actor%20Object%20Reference))
  (|CallParentFunction OtherActor) ; This node is disabled and will not be called.\nDrag off pins to build functionality.
)

(event EventTick
  (params (DeltaSeconds :type Float%20%28single-precision%29))
  (|CallParentFunction DeltaSeconds) ; This node is disabled and will not be called.\nDrag off pins to build functionality.
)

(fn ConstructionScript
  (|CallParentFunction))