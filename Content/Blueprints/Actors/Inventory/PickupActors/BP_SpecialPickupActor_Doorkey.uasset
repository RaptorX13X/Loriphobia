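; Pickup actor for a door key that the player collects with the action input.
; Pressing the action increments the player's collected key count, then adds the item to the player's inventory component.
; A partial add leaves the remaining amount on the pickup, while a full add plays a random 2D sound and destroys the actor.
; The key count rises on every press, even if the inventory add fails.
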(event Input|ActionEvents|InputActionAction
  (params (Key :type Key%20Structure :default "None"))
  (bind _player_ref (Variables|Default|GetPlayer%20Ref))
  (:Pressed
    (Variables|/Game/Blueprints/Game/Level1/L1_Character.L1_Character_C|SetKeyCollected _player_ref (+ (Variables|/Game/Blueprints/Game/Level1/L1_Character.L1_Character_C|GetKeyCollected _player_ref) 1))
    (bind (_success_ _remainder) (Default|AddItem (Variables|/Game/Blueprints/Game/Level1/L1_Character.L1_Character_C|GetBPC_Inventory _player_ref) (Variables|Default|GetItem) (Variables|Default|GetAmount)))
    (if _success_
      (if (> _remainder 0)
        (Variables|Default|SetAmount _remainder)
        (else
          (Audio|PlaySound2D (.OutItem (Utilities|Array|Random (Variables|Default|GetSound))) 1.0 1.0 0.0 0 0)
          (Actor|DestroyActor))))))

(fn ConstructionScript
  (|CallParentFunction))